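; Actor component that lets the owning first-person character vault onto ledges.
; While idle, Tick traces down ahead of the character, validates ledge height, walkable slope and capsule clearance, then stores the landing point and adds a vault widget to the viewport.
; Vault switches the state, after which Tick lerps the character to that point by teleporting without sweep, then resets.
; Debug drawing and prints are left on.
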(event `self.ReceiveBeginPlay`
  (bind _asbp_first_person_character (cast `/Game/StarterContent/FirstPerson/Blueprints/BP_FirstPersonCharacter` (`self.GetOwner`)))
  (set `self.Owning Character` _asbp_first_person_character)
  (bind _returnvalue (`|CreateWidget` "/Game/Blueprints/Vaulting/Vault_Widget.Vault_Widget_C" (cast `PlayerController` (`Pawn.GetController` (`self.Owning Character`)) :!pure true)))
  (set `self.Vault Widget` _returnvalue))

(event `self.ReceiveTick`
  (params (DeltaSeconds :type "Float (single-precision)"))
  (`self.SwitchVaultingState`
    (:`NotVaulting `
      (bind (_result _ending_location) (`self.Can Vault`))
      (if _result
        (set `self.Ending Location` _ending_location)
        (if (not (`Widget.IsInViewport` (`self.Vault Widget`)))
          (`UserWidget.AddToViewport` (`self.Vault Widget`) 0))
        (elif (not (`Widget.IsInViewport` (`self.Vault Widget`)))
          (`Widget.RemoveFromParent` (`self.Vault Widget`)))))
    (:`Vaulting`
      (`self.TickVault` DeltaSeconds))))

(event `Vault`
  (set `self.Progress` 0.0)
  (set `self.StartingLocation` (`Actor.K2_GetActorLocation` (`self.Owning Character`)))
  (set `self.Vaulting State` "NewEnumerator2"))

(fn `Can Vault`
  (returns (Result :type Boolean) (`Ending Location` :type "Vector Structure"))
  (locals (`Capsule (Local)` :type "CapsuleComponent Object Reference"))
  (bind _owning_character (`self.Owning Character`))
  (bind _returnvalue (`CapsuleComponent.GetScaledCapsuleHalfHeight` (`local.Capsule (Local)`)))
  (bind _returnvalue_2 (+ (`Actor.K2_GetActorLocation` _owning_character) (* (`Actor.GetActorForwardVector` _owning_character) 70.0)))
  (if (`|EnumEquality` (`self.Vaulting State`) "NewEnumerator0")
    (set `local.Capsule (Local)` (`Character.CapsuleComponent` (`self.Owning Character`)))
    (bind (_outhit _returnvalue_3) (`KismetSystemLibrary.LineTraceSingle` (+ _returnvalue_2 (`KismetMathLibrary.MakeVector` 0.0 0.0 _returnvalue)) (- _returnvalue_2 (`KismetMathLibrary.MakeVector` 0.0 0.0 _returnvalue)) "TraceTypeQuery1" false (`|MakeArray` (`self.Owning Character`) :!type "Actor Object Reference") "ForOneFrame"))
    (if _returnvalue_3
      (bind (_result _endinglocation) (`self.CanVaultToHit` (`local.Capsule (Local)`) _outhit))
      (`KismetSystemLibrary.PrintString` (`KismetStringLibrary.Conv_BoolToString` _result) true true (struct :`G` 0.66 :`B` 1.0 :`A` 1.0) 0.0)
      (return _result _endinglocation)
      (else
        (return false (0.0 0.0 0.0))))
    (else
      (return false (0.0 0.0 0.0)))))

(fn `CanVaultToHit`
  (params (Capsule :type "CapsuleComponent Object Reference") (Hit :type "HitResult Structure"))
  (returns (Result :type Boolean) (EndingLocation :type "Vector Structure"))
  (locals (`EndingLocation (Local)` :type "Vector Structure" :default (0.0 0.0 0.0)))
  (bind (_hit_bblockinghit _hit_binitialoverlap _hit_time _hit_distance _hit_location) (`GameplayStatics.BreakHitResult` (`local.Hit`)))
  (bind (_hit_bblockinghit_2 _hit_binitialoverlap_2 _hit_time_2 _hit_distance_2 _hit_location_2 _hit_impactpoint _hit_normal _hit_impactnormal _hit_physmat _hit_hitactor _hit_hitcomponent _hit_hitbonename _hit_bonename _hit_hititem _hit_elementindex _hit_faceindex _hit_tracestart _hit_traceend) (`GameplayStatics.BreakHitResult` (`local.Hit`)))
  (bind (_hit_bblockinghit_3 _hit_binitialoverlap_3 _hit_time_3 _hit_distance_3 _hit_location_3 _hit_impactpoint_2 _hit_normal_2) (`GameplayStatics.BreakHitResult` (`local.Hit`)))
  (bind _capsule (`local.Capsule`))
  (bind _returnvalue (`CapsuleComponent.GetScaledCapsuleRadius` _capsule))
  (bind _returnvalue_2 (- (.z _hit_location_2) (.z _hit_traceend)))
  (`|ExecutionSequence`
    (:`then_0`
      ;[0.3221 0.8482 1] Make Sure that Ledge is at an Appropriate Height
      (`KismetSystemLibrary.PrintString` (`KismetStringLibrary.Conv_DoubleToString` _returnvalue_2) true true (struct :`G` 0.66 :`B` 1.0 :`A` 1.0) 0.0)
      (if (not (`KismetMathLibrary.InRange_FloatFloat` _returnvalue_2 (`self.MinVautingHeight`) (`self.MaxVautingHeight`)))
        (return false (0.0 0.0 0.0))))
    (:`then_1`
      ;[0.6659 1 0.1118] Make Sure the surface we're vaulting to is walkable
      (if (< (.z _hit_normal_2) (`CharacterMovementComponent.K2_GetWalkableFloorZ` (`Character.CharacterMovement` (`self.Owning Character`))))
        (return false (0.0 0.0 0.0))))
    (:`then_2`
      ;[1 0.04211 0.04211] Make sure that there is room for character on top of leadge
      (bind _output_get (set `local.EndingLocation (Local)` (+ _hit_location (`KismetMathLibrary.MakeVector` 0.0 0.0 (`CapsuleComponent.GetScaledCapsuleHalfHeight` (`local.Capsule`))))))
      (bind _result (`self.CheckCapsuleCollison` (+ _output_get (`KismetMathLibrary.MakeVector` 0.0 0.0 _returnvalue)) (`CapsuleComponent.GetScaledCapsuleHalfHeight` _capsule) _returnvalue true))
      (if _result
        (return false (0.0 0.0 0.0))))
    (:`then_3`
      (return true (`local.EndingLocation (Local)`)))))

(fn `CheckCapsuleCollison`
  (params (Center :type "Vector Structure") (`Half Height` :type "Float (double-precision)") (Radius :type "Float (double-precision)") (`Draw Debug` :type Boolean))
  (returns (Result :type Boolean))
  (`|ExecutionSequence`
    (:`then_0`
      (if (`local.Draw Debug`)
        (`KismetSystemLibrary.DrawDebugCapsule` (`local.Center`) (`local.Half Height`) (`local.Radius`) (struct) (struct :`R` 0.01269 :`G` 0.188371 :`B` 1.0 :`A` 1.0) 0.0 3.0)))
    (:`then_1`
      (bind (_outactors _returnvalue) (`KismetSystemLibrary.CapsuleOverlapActors` (`local.Center`) (`local.Radius`) (`local.Half Height`) (`|MakeArray` "ObjectTypeQuery1" :!type "EObjectTypeQuery Enum") "/Script/Engine.Actor" (`|MakeArray` (`self.Owning Character`) :!type "Actor Object Reference")))
      (return _returnvalue))))

(fn `Get Vaulting state`
  (returns (`Vaulting State` :type "/Game/Blueprints/Vaulting/EVaultingState Enum"))
  (return (`self.Vaulting State`)))

(fn `TickVault`
  (params (`Delta Seconds` :type "Float (double-precision)"))
  (`|ExecutionSequence`
    (:`then_0`
      (set `self.Progress` (`KismetMathLibrary.FClamp` (+ (`self.Progress`) (/ (`local.Delta Seconds`) (`self.VaultSpeed`)))))
      (`Actor.K2_SetActorLocation` (`self.Owning Character`) (`KismetMathLibrary.VLerp` (`self.StartingLocation`) (`self.Ending Location`) (`self.Progress`)) false true))
    (:`then_1`
      (if (>= (`self.Progress`) 1.0)
        (set `self.Vaulting State` "NewEnumerator0")))))