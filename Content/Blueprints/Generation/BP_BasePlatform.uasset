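; Base platform actor for procedural chunk generation, with a random mesh picked at construction and a lifespan staggered by grid number.
; Outside chunk zero, its mesh starts raised by grid number, and Tick drops the actor until the mesh matches its original location exactly.
; A player hit on the platform at grid index max minus two asks the game mode for new chunks, first clearing that trigger on platforms sharing its grid-number tag.
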(event `self.ReceiveBeginPlay`
  (`|ExecutionSequence`
    (:`then_0`
      (if (not (== (`self.ChunkNumber`) 0))
        (set `self.InitialLocation` (`SceneComponent.K2_GetComponentLocation` (`self.PlatformMesh`)))
        (`SceneComponent.K2_AddWorldOffset` (`self.PlatformMesh`) (`KismetMathLibrary.MakeVector` 0.0 0.0 (* (`self.GridNumber`) (`self.HeightOffset`))) false false)
        (set `self.ShouldFall` true)))
    (:`then_1`
      (`KismetArrayLibrary.Array_Add` (`self.Tags`) (`KismetStringLibrary.Conv_StringToName` (`KismetStringLibrary.Conv_IntToString` (`self.GridNumber`)))))
    (:`then_2`
      (if (== (`self.GridNumber`) (- (`self.MaxNumberOfGridsPerChunk`) 2))
        (set `self.ShouldSpawnChunk` true)))
    (:`then_3`
      (`KismetSystemLibrary.Delay` (+ (`self.GridNumber`) (`self.Lifespan`)))
      (`self.K2_DestroyActor`))))

(event `self.ReceiveTick`
  (params (DeltaSeconds :type "Float (single-precision)"))
  (if (`self.ShouldFall`)
    (`self.K2_AddActorWorldOffset` (0.0 0.0 -50.0) false true)
    (if (== (`SceneComponent.K2_GetComponentLocation` (`self.PlatformMesh`)) (`self.InitialLocation`))
      (set `self.ShouldFall` false))))

(event `self.ReceiveHit`
  (params (MyComp :type "PrimitiveComponent Object Reference") (Other :type "Actor Object Reference") (OtherComp :type "PrimitiveComponent Object Reference") (bSelfMoved :type Boolean) (HitLocation :type "Vector Structure") (HitNormal :type "Vector Structure") (NormalImpulse :type "Vector Structure") (Hit :type "HitResult Structure (by ref)"))
  (`KismetSystemLibrary.PrintString` (`KismetStringLibrary.Concat_StrStr` "Grid Number: " (`KismetStringLibrary.Conv_IntToString` (`self.GridNumber`)) "Should Spawn Chunk: " (`KismetStringLibrary.Conv_BoolToString` (`self.ShouldSpawnChunk`))))
  (if (`self.ShouldSpawnChunk`)
    (cast `/Game/Blueprints/BP_FirstPersonCharacter` Other)
    ;[1 1 1] shits ass but it works some of the time so thats fine
    (bind _outactors (`GameplayStatics.GetAllActorsOfClassWithTag` "BP_BasePlatform_C" (`KismetStringLibrary.Conv_StringToName` (`KismetStringLibrary.Conv_IntToString` (`self.GridNumber`)))))
    (for _array_element _outactors
      (set `/Game/Blueprints/Generation/BP_BasePlatform.ShouldSpawnChunk` false _array_element))
    (`/Game/Blueprints/BP_BugginOutGameMode.SpawnNewChunks` (`/Game/Blueprints/FL_GeneralFunctionLibrary.GetBugginOutGameMode`))))

(fn `UserConstructionScript`
  (`StaticMeshComponent.SetStaticMesh` (`self.PlatformMesh`) (`KismetArrayLibrary.Array_Random` (`self.MeshArray`))))