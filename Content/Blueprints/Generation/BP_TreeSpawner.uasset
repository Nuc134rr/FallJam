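; BP_TreeSpawner builds the tree by spawning stacked trunk segments in chunks.
; On BeginPlay it spawns a base tree to measure trunk size, spawns a first chunk and binds SpawnTrunks to the game mode's new-chunk event.
; Each segment class comes from the weighted TrunkClasses map: a roll up to the weight sum shortlists classes weighted above it, then one is chosen randomly.
; Segment height depends only on loop index; the computed HeightOffest is unused.
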(event `SetOffsetVariables`
  (`|ExecutionSequence`
    (:`then_0`
      (bind _returnvalue (`|SpawnActorFromClass` "/Game/Blueprints/Generation/BP_BaseTree.BP_BaseTree_C" (`KismetMathLibrary.MakeTransform` (0.0 0.0 0.0)) "Undefined" "OverrideRootScale" null null))
      (bind (_origin _boxextent) (`KismetSystemLibrary.GetComponentBounds` (`/Game/Blueprints/Generation/BP_BaseTree.TreeMesh` _returnvalue)))
      (set `self.TrunkDiameter` (* (.x _boxextent) 2.0))
      (set `self.TrunkHeight` (* (.z _boxextent) 2.0)))
    (:`then_1`
      (set `self.HeightOffest` (* (`self.MaxSpawnedTrunksPerChunk`) (`self.TrunkHeight`))))))

(event `self.ReceiveBeginPlay`
  (`|ExecutionSequence`
    (:`then_0`
      (`self.SetOffsetVariables`))
    (:`then_1`
      (`self.SpawnTrunks`))
    (:`then_2`
      (add `/Game/Blueprints/BP_BugginOutGameMode.SpawnNewChunks` (`/Game/Blueprints/FL_GeneralFunctionLibrary.GetBugginOutGameMode`) (delegate `SpawnTrunks`)))))

(event `SpawnTrunks`
  (for _index (range (+ (`self.MaxSpawnedTrunksPerChunk`) 1))
    (bind _percentagesum (`self.CalculatePlatformSum`))
    (bind _trunkclass (`self.PickTreeTrunk` _percentagesum))
    (`|SpawnActorFromClass` _trunkclass (`KismetMathLibrary.MakeTransform` (`KismetMathLibrary.MakeVector` 0.0 0.0 (* (+ _index 1) (`self.TrunkHeight`)))) "Undefined" "OverrideRootScale" null null)))

(fn `CalculatePlatformSum`
  (returns (PercentageSum :type "Float (double-precision)"))
  (locals (PercSum :type "Float (double-precision)"))
  (bind _values (`BlueprintMapLibrary.Map_Values` (`self.TrunkClasses`)))
  (for _array_element _values
    (set `local.PercSum` (+ _array_element (`local.PercSum`))))
  (return (`local.PercSum`)))

(fn `PickTreeTrunk`
  (params (PercentageSum :type "Float (double-precision)"))
  (returns (TrunkClass :type "/Game/Blueprints/Generation/BP_BaseTree Class Reference"))
  (locals (RandomFloat :type "Float (double-precision)" :default 0.0) (PossibleTrunkArray :type "Array of /Game/Blueprints/Generation/BP_BaseTree Class Reference"))
  (bind _trunkclasses (`self.TrunkClasses`))
  (set `local.RandomFloat` (`KismetMathLibrary.RandomFloatInRange` 0.0 (`local.PercentageSum`)))
  (bind _keys (`BlueprintMapLibrary.Map_Keys` _trunkclasses))
  (for _array_element _keys
    (if (< (`local.RandomFloat`) (`BlueprintMapLibrary.Map_Find` _trunkclasses _array_element))
      (`KismetArrayLibrary.Array_Add` (`local.PossibleTrunkArray`) _array_element)))
  (return (`KismetArrayLibrary.Array_Random` (`local.PossibleTrunkArray`))))

(fn `UserConstructionScript`)