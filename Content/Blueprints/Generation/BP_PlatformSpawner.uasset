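; Platform spawner actor that builds a stack of platform grids at BeginPlay, rising in height and stepping around the Z axis in a spiral.
; It measures tile size from a temporarily spawned platform's mesh bounds, then spawns each tile with its grid, row and column numbers.
; Tile classes come from a weighted map: a roll up to the weight total picks the first entry whose own, non-cumulative weight exceeds it.
; TransformGrid can shift existing platforms, but nothing here calls it.
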(event `SetOffsetVariables`
  ;[1 0.2 0.2] Set Offset Variables
  (`|ExecutionSequence`
    (:`then_0`
      (bind _keys (`BlueprintMapLibrary.Map_Keys` (`self.PlatformClasses`)))
      (bind _returnvalue (`|SpawnActorFromClass` (`|GetArrayItem` _keys) (`KismetMathLibrary.MakeTransform` (0.0 0.0 0.0)) "Undefined" "OverrideRootScale" null 0 0 0 null))
      (set `self.TileSize` (* (.x (`.BoxExtent` (`KismetSystemLibrary.GetComponentBounds` (`/Game/Blueprints/Generation/BP_BasePlatform.PlatformMesh` _returnvalue)))) 2.0))
      (`self.K2_DestroyActor` _returnvalue))
    (:`then_1`
      (set `self.XOffset` (* (`self.NumberOfPlatformColumns`) (`self.TileSize`)))
      (set `self.YOffset` (* (`self.NumberOfPlatformRows`) (`self.TileSize`))))))

(event `self.ReceiveBeginPlay`
  (`|ExecutionSequence`
    (:`then_0`
      (`self.SetOffsetVariables`))
    (:`then_1`
      (for _ (range (+ (`self.MaxNumberOfGrids`) 1))
        (`KismetSystemLibrary.PrintString` "Hello")
        (`self.CreateGrid`)
        (`/Engine/EditorBlueprintResources/StandardMacros.IncrementInt` (`self.GridsSpawned`))))))

(event `CreateGrid`
  (bind _tilesize (`self.TileSize`))
  ;[0.2 0.2 0.2] Create Gird for Platforms
  (for _index (range (+ (`self.NumberOfPlatformRows`) 1))
    (for _index_2 (range (+ (`self.NumberOfPlatformColumns`) 1))
      (bind _percentagesum (`self.CalculatePlatformPercent`))
      (bind _platformclass (`self.PickPlatform` _percentagesum))
      (`|SpawnActorFromClass` _platformclass (`KismetMathLibrary.MakeTransform` (+ (`KismetMathLibrary.MakeVector` (* _index_2 _tilesize) (* _index _tilesize) (* (`self.GridsSpawned`) (`self.HeightOffset`))) (`KismetMathLibrary.RotateAngleAxis` (`KismetMathLibrary.MakeVector` (`self.Radius`)) (* (`self.GridsSpawned`) (`self.AngleOffset`)) (0.0 0.0 1.0))) (`KismetMathLibrary.MakeRotator` 0.0)) "Undefined" "OverrideRootScale" null (+ (`self.GridsSpawned`) 1) _index _index_2 null))))

(fn `CalculatePlatformPercent`
  (returns (PercentageSum :type "Float (double-precision)"))
  (locals (PercSum :type "Float (double-precision)"))
  (bind _values (`BlueprintMapLibrary.Map_Values` (`self.PlatformClasses`)))
  (for _array_element _values
    (set `local.PercSum` (+ _array_element (`local.PercSum`))))
  (return (`local.PercSum`)))

(fn `PickPlatform`
  (params (PercentageSum :type "Float (double-precision)"))
  (returns (PlatformClass :type "/Game/Blueprints/Generation/BP_BasePlatform Class Reference"))
  (locals (PlatformToSpawn :type "/Game/Blueprints/Generation/BP_BasePlatform Class Reference") (RandomFloat :type "Float (double-precision)" :default 0.0))
  (bind _platformclasses (`self.PlatformClasses`))
  (set `local.RandomFloat` (`KismetMathLibrary.RandomFloatInRange` 0.0 (`local.PercentageSum`)))
  (bind _keys (`BlueprintMapLibrary.Map_Keys` _platformclasses))
  (for _array_element _keys
    (if (< (`local.RandomFloat`) (`BlueprintMapLibrary.Map_Find` _platformclasses _array_element))
      (set `local.PlatformToSpawn` _array_element)
      (break)))
  (return (`local.PlatformToSpawn`)))

(fn `TransformGrid`
  (params (CurrentGridPlatforms :type "Array of /Game/Blueprints/Generation/BP_BasePlatform Object Reference"))
  (for _array_element CurrentGridPlatforms
    (`self.K2_AddActorWorldOffset` _array_element (`KismetMathLibrary.RotateAngleAxis` (2000.0 0.0 0.0) (* (`self.AngleOffset`) (`self.GridsSpawned`)) (0.0 0.0 1.0)) false true)))

(fn `UserConstructionScript`)