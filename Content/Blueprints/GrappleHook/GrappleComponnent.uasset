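; Grapple component that launches a grappling hook projectile from its owner toward a target location.
; A state enum (ready, firing, attached) gates firing, so FireGrapple spawns BP_GrappleHook only when idle, with velocity along the normalized direction from the cable start point.
; CancelGrapple is an empty stub, and the Cable Start Location graph's owner-relative offset calculation is left unconnected.
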(fn `Cancel Grapple`)

(fn `fireGrapple`
  (params (`Target Location` :type "Vector Structure") (LocalOffset :type "Vector Structure"))
  (locals (FireDirection :type "Vector Structure" :default (0.0 0.0 0.0)))
  (if (not (`self.IsInUse?`))
    (set `self.GrappleState` "NewEnumerator1")
    (set `local.FireDirection` (`KismetMathLibrary.Normal` (- (`local.Target Location`) (`self.Cable Start Location` (`local.LocalOffset`)))))
    (`|SpawnActorFromClass` "/Game/Blueprints/GrappleHook/BP_GrappleHook.BP_GrappleHook_C" (`KismetMathLibrary.MakeTransform` (`self.Cable Start Location` (`local.LocalOffset`))) "Undefined" "OverrideRootScale" null (* (`local.FireDirection`) (`self.Speed`)) null)))

(fn `IsInUse?`
  (returns (result :type Boolean))
  (return (select `/Game/Blueprints/GrappleHook/EGrappleState` (`self.GrappleState`) :`NewEnumerator1` true :`NewEnumerator2` true)))